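; MyMain is the player character Blueprint, handling noise emission, animation state and pausing.
; A looping timer started on BeginPlay makes regular pawn noise, detectable by AI sensing.
; Each Tick pushes its States value to FurFurAnimationBP, overridden with Dead when PlayerDead is set.
; The Pause input freezes the game and shows a reused menu widget with UI-only input, while Unpausegame clears widgets and restores game input.
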(event `FSNoise`
  (`self.PawnMakeNoise` 1.0 (0.0 0.0 0.0) true self))

(event `self.ReceiveBeginPlay`
  (`KismetSystemLibrary.K2_SetTimer` null "FSNoise" 0.5 true))

(event `self.ReceiveTick`
  (params (DeltaSeconds :type "Float (single-precision)"))
  (bind _asfur_fur_animation_bp (cast `/Game/Animation/FurFurAnimations/FurFurAnimationBP` (`SkeletalMeshComponent.GetAnimInstance` (`self.Mesh`))))
  (if (`self.bPlayerDead`)
    (set `/Game/Animation/FurFurAnimations/FurFurAnimationBP.animationStates` "dead" _asfur_fur_animation_bp)
    (else
      (set `/Game/Animation/FurFurAnimations/FurFurAnimationBP.animationStates` (`self.states`) _asfur_fur_animation_bp))))

(event `InputAction|Pause`
  (params (Key :type "Key Structure"))
  (:`Pressed`
    (`self.Pausegame`)))

(fn `Pausegame`
  (`GameplayStatics.SetGamePaused` true)
  (`/Engine/EditorBlueprintResources/StandardMacros.IsValid` (`self.pausemenu`)
    (:`Is Valid`
      _)
    (:`Is Not Valid`
      (bind _returnvalue (`|CreateWidget` "/Game/UI/Pausemenu/Pausemenu.Pausemenu_C" (`GameplayStatics.GetPlayerController` 0)))
      (set `self.pausemenu` _returnvalue)))
  (`UserWidget.AddToViewport` (`self.pausemenu`) 0)
  (`WidgetBlueprintLibrary.SetInputMode_UIOnlyEx` (`GameplayStatics.GetPlayerController` 0) (`self.pausemenu`))
  (set `PlayerController.bShowMouseCursor` true (`GameplayStatics.GetPlayerController` 0)))

(fn `Unpausegame`
  (bind _returnvalue (`GameplayStatics.GetPlayerController` 0))
  (`GameplayStatics.SetGamePaused` false)
  (`WidgetLayoutLibrary.RemoveAllWidgets`)
  (`WidgetBlueprintLibrary.SetInputMode_GameOnly` _returnvalue)
  (set `PlayerController.bShowMouseCursor` false _returnvalue))

(fn `UserConstructionScript`)